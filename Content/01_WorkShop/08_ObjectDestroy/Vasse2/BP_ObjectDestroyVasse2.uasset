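; Breakable vase that swaps its static mesh for a fractured version when it hits the floor.
; A sphere overlap with an actor tagged "Floor" fires once, hiding the mesh and disabling its collision.
; It spawns BP_Vase2_GeometryCollection at the same transform, then after a short delay plays a sound at its location and disables the sphere's collision.
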(event OnComponentBeginOverlap(Sphere)
  (params (OverlappedComponent :type Primitive%20Component%20Object%20Reference) (OtherActor :type Actor%20Object%20Reference) (OtherComp :type Primitive%20Component%20Object%20Reference) (OtherBodyIndex :type Integer) (bFromSweep :type Boolean) (SweepResult :type Hit%20Result%20Structure%20%28by%20ref%29))
  (if (Actor|ActorHasTag OtherActor "Floor")
    (Utilities|FlowControl|DoOnce false
      (:Completed
        (Utilities|FlowControl|Sequence
          (:then_0
            ;[1 1 1] SetStaticMeshFalseVisibility
            (|SetStaticMeshFalseVisibility))
          (:then_1
            (Game|SpawnActorfromClass "/Game/01_WorkShop/08_ObjectDestroy/Vasse2/RequiredItems/BP_Vase2_GeometryCollection.BP_Vase2_GeometryCollection_C" (Transformation|GetActorTransform) "Undefined" 0 0)
            (Utilities|FlowControl|Delay 0.1)
            (Audio|SpawnSoundatLocation "/Game/01_WorkShop/08_ObjectDestroy/Vasse1/RequiredItems/1531.1531" (Transformation|GetActorLocation) "0, 0, 0" 1.0 1.0 0.0 0 0)
            (Collision|SetCollisionEnabled (Variables|Default|GetSphere) "NoCollision")))))))

(event Collision|EventActorBeginOverlap
  (params (OtherActor :type Actor%20Object%20Reference)))

(event EventTick
  (params (DeltaSeconds :type Float%20%28single-precision%29)))

(fn ConstructionScript)