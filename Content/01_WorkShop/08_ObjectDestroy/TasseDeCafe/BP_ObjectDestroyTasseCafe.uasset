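; Destructible coffee cup actor that shatters and awards score when its sphere overlaps an actor tagged Floor.
; A one-time trigger hides the static mesh and spawns a Geometry Collection replacement at the same transform.
; After a brief delay it plays a sound, disables sphere collision and adds its Value to the HUD_test score.
; The HUD reference is cached on actor overlap rather than at BeginPlay.
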(event OnComponentBeginOverlap(Sphere)
  (params (OverlappedComponent :type Primitive%20Component%20Object%20Reference) (OtherActor :type Actor%20Object%20Reference) (OtherComp :type Primitive%20Component%20Object%20Reference) (OtherBodyIndex :type Integer) (bFromSweep :type Boolean) (SweepResult :type Hit%20Result%20Structure%20%28by%20ref%29))
  (bind _hud_test (Variables|Default|GetHUD%20Test))
  (if (Actor|ActorHasTag OtherActor "Floor")
    (Utilities|FlowControl|DoOnce false
      (:Completed
        (Utilities|FlowControl|Sequence
          (:then_0
            ;[1 1 1] SetStaticMeshFalseVisibility
            (|SetStaticMeshFalseVisibility))
          (:then_1
            (Game|SpawnActorfromClass "/Game/01_WorkShop/08_ObjectDestroy/TasseDeCafe/RequiredItems/BP_TasseCafe_GeometryCollection.BP_TasseCafe_GeometryCollection_C" (Transformation|GetActorTransform) "Undefined" "OverrideRootScale" 0 0)
            (Utilities|FlowControl|Delay 0.1)
            (Audio|SpawnSoundatLocation "/Game/01_WorkShop/08_ObjectDestroy/TasseDeCafe/RequiredItems/16648.16648" (Transformation|GetActorLocation) "0, 0, 0" 1.0 1.0 0.0 0 0)
            (Collision|SetCollisionEnabled (Variables|Default|GetSphere) "NoCollision")
            (Utilities|IsValid _hud_test
              (:Is%20Valid
                (Default|AddScore _hud_test (Variables|Default|GetValue))))))))))

(event Collision|EventActorBeginOverlap
  (params (OtherActor :type Actor%20Object%20Reference))
  (bind _ashud_test (Utilities|Casting|CastToHUD_test (HUD|GetHUD (Game|GetPlayerController 0))))
  (Variables|Default|SetHUD%20Test _ashud_test))

(event EventTick
  (params (DeltaSeconds :type Float%20%28single-precision%29)))

(fn ConstructionScript)