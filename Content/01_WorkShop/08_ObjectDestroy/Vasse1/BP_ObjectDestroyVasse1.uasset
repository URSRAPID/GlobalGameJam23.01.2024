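; A breakable vase prop that shatters when its sphere trigger overlaps an actor tagged Floor.
; On that overlap, once only, it hides and disables the static mesh, spawns a Geometry Collection vase at its transform and plays a glass-breaking sound.
; It then adds its Value to the HUD score and flags the destroyed object's name on the player character, both cached at BeginPlay.
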(event OnComponentBeginOverlap(Sphere)
  (params (OverlappedComponent :type Primitive%20Component%20Object%20Reference) (OtherActor :type Actor%20Object%20Reference) (OtherComp :type Primitive%20Component%20Object%20Reference) (OtherBodyIndex :type Integer) (bFromSweep :type Boolean) (SweepResult :type Hit%20Result%20Structure%20%28by%20ref%29))
  (bind _hud_test (Variables|Default|GetHUD%20Test))
  (bind _as_c_perso (Variables|Default|GetAs%20C%20Perso))
  (if (Actor|ActorHasTag OtherActor "Floor")
    (Utilities|FlowControl|DoOnce false
      (:Completed
        (Utilities|FlowControl|Sequence
          (:then_0
            ;[1 1 1] SetStaticMeshFalseVisibility
            (|SetStaticMeshFalseVisibility))
          (:then_1
            (Game|SpawnActorfromClass "/Game/01_WorkShop/08_ObjectDestroy/Vasse1/RequiredItems/BP_Vase1_GeometryCollection.BP_Vase1_GeometryCollection_C" (Transformation|GetActorTransform) "Undefined" "OverrideRootScale" 0 0)
            (Utilities|FlowControl|Delay 0.1)
            (Audio|SpawnSoundatLocation "/Game/01_WorkShop/08_ObjectDestroy/SoundVerreAll/040683_breaking-glass-75142__mp3cut_net___2__Cue.040683_breaking-glass-75142__mp3cut_net___2__Cue" (Transformation|GetActorLocation) "0, 0, 0" 1.0 1.0 0.0 0 0)
            (Collision|SetCollisionEnabled (Variables|Default|GetSphere) "NoCollision")
            (Utilities|FlowControl|Sequence
              (:then_0
                (Utilities|IsValid _hud_test
                  (:Is%20Valid
                    (Default|AddScore _hud_test (Variables|Default|GetValue)))))
              (:then_1
                (Variables|/Game/01_WorkShop/02_Core/C_Perso.C_Perso_C|SetNameObjectDestroy _as_c_perso (Variables|Default|GetVasse1))
                (Variables|/Game/01_WorkShop/02_Core/C_Perso.C_Perso_C|SetDestroy%20object%20? _as_c_perso true)))))))))

(event EventBeginPlay
  (bind _ashud_test (Utilities|Casting|CastToHUD_test (HUD|GetHUD (Game|GetPlayerController 0))))
  (Variables|Default|SetHUD%20Test _ashud_test)
  (bind _asc_perso (Utilities|Casting|CastToC_Perso (Game|GetPlayerCharacter 0)))
  (Variables|Default|SetAs%20C%20Perso _asc_perso))

(event EventTick
  (params (DeltaSeconds :type Float%20%28single-precision%29)))

(fn ConstructionScript)