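; BP_ObjectDestroy is a breakable object that swaps its static mesh for a champagne set Geometry Collection when it touches the floor.
; A Sphere overlap with an actor tagged "Floor" hides the mesh and disables its collision, then immediately spawns BP_champagneSet1_GeometryCollection at the actor's transform.
; The one-second Delay after hiding leads to nothing, debug strings print along the way, and the original actor is never destroyed.
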(event OnComponentBeginOverlap(Sphere)
  (params (OverlappedComponent :type Primitive%20Component%20Object%20Reference) (OtherActor :type Actor%20Object%20Reference) (OtherComp :type Primitive%20Component%20Object%20Reference) (OtherBodyIndex :type Integer) (bFromSweep :type Boolean) (SweepResult :type Hit%20Result%20Structure%20%28by%20ref%29))
  (if (Actor|ActorHasTag OtherActor "Floor")
    (Development|PrintString "Hello")
    (Utilities|FlowControl|Sequence
      (:then_0
        ;[1 1 1] SetStaticMeshFalseVisibility
        (|SetStaticMeshFalseVisibility))
      (:then_1
        (Development|PrintString "OK")
        (Game|SpawnActorfromClass "/Game/01_WorkShop/08_ObjectDestroy/BP_champagneSet1_GeometryCollection.BP_champagneSet1_GeometryCollection_C" (Transformation|GetActorTransform) "Undefined" 0 0)))))

(event EventBeginPlay)

(event Collision|EventActorBeginOverlap
  (params (OtherActor :type Actor%20Object%20Reference)))

(event EventTick
  (params (DeltaSeconds :type Float%20%28single-precision%29)))

(fn ConstructionScript)