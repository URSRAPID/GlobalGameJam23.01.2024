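; Respawn trigger volume, kept in a Test folder, that sends the player back to their start point.
; Any overlap with its box disables input on player 0's pawn, moves it without sweep to the StartLocation stored on C_Perso, then re-enables input.
; The overlapping actor is never checked, and a failed C_Perso cast leaves input disabled.
; The construction script sizes the box from the InBoxExtent variable.
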(event OnComponentBeginOverlap(Box)
  (params (OverlappedComponent :type Primitive%20Component%20Object%20Reference) (OtherActor :type Actor%20Object%20Reference) (OtherComp :type Primitive%20Component%20Object%20Reference) (OtherBodyIndex :type Integer) (bFromSweep :type Boolean) (SweepResult :type Hit%20Result%20Structure%20%28by%20ref%29))
  (bind _returnvalue (Game|GetPlayerController 0))
  (bind _returnvalue_2 (Pawn|GetControlledPawn _returnvalue))
  (Input|DisableInput _returnvalue_2 0)
  (bind _asc_perso (Utilities|Casting|CastToC_Perso _returnvalue_2))
  (Transformation|SetActorLocation _returnvalue_2 (Variables|/Game/01_WorkShop/02_Core/C_Perso.C_Perso_C|GetStartLocation _asc_perso) false false)
  (Input|EnableInput _returnvalue_2 0))

(event EventBeginPlay)

(event Collision|EventActorBeginOverlap
  (params (OtherActor :type Actor%20Object%20Reference)))

(event EventTick
  (params (DeltaSeconds :type Float%20%28single-precision%29)))

(fn ConstructionScript
  (Components|Box|SetBoxExtent (Variables|Default|GetBox) (Variables|Default|GetIn%20Box%20Extent) true))