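; BP_Platform_2 is a placeable moving platform that shuttles endlessly between its local origin and a configurable PhantomLocation offset.
; On BeginPlay, a FlipFlop picks each target for a looping, eased MoveComponentTo lasting Period.
; The Construction Script tints Platform and Phantom through dynamic materials using Color.
; It also previews the path, placing Phantom at the rotated endpoint and aiming and stretching Arrow toward it.
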(event EventBeginPlay
  (bind _isa (Utilities|FlowControl|FlipFlop :!label _label)
    (:A
      _)
    (:B
      _))
  (Components|MoveComponentTo (Variables|Default|GetPlatform) (Math|Vector|SelectVector (Variables|Default|GetPhantomLocation) "0, 0, 0" _isa) "0, 0, 0" true true (Variables|Default|GetPeriod) false)
  (goto _label))

(event Collision|EventActorBeginOverlap
  (params (OtherActor :type Actor%20Object%20Reference)))

(event EventTick
  (params (DeltaSeconds :type Float%20%28single-precision%29)))

(fn ConstructionScript
  (bind _color (Variables|Default|GetColor))
  (bind _platform (Variables|Default|GetPlatform))
  (bind _phantom (Variables|Default|GetPhantom))
  (bind _arrow (Variables|Default|GetArrow))
  (bind _returnvalue (Transformation|GetWorldLocation _phantom))
  (bind _returnvalue_2 (Transformation|GetWorldLocation _platform))
  (Utilities|FlowControl|Sequence
    (:then_0
      (Utilities|FlowControl|Sequence
        (:then_0
          (bind _returnvalue_3 (Rendering|Material|CreateDynamicMaterialInstance (Variables|Default|GetPlatform) 0 "/Game/01_WorkShop/03_Pacebles/Platform/M_Platform.M_Platform" "None" :!class /Script/Engine.PrimitiveComponent))
          (Rendering|Material|SetVectorParameterValue _returnvalue_3 "Color" _color :!class /Script/Engine.MaterialInstanceDynamic))
        (:then_1
          (bind _returnvalue_4 (Rendering|Material|CreateDynamicMaterialInstance (Variables|Default|GetPhantom) 0 "/Game/01_WorkShop/03_Pacebles/Platform/M_Platform_2.M_Platform_2" "None" :!class /Script/Engine.PrimitiveComponent))
          (Rendering|Material|SetVectorParameterValue _returnvalue_4 "Color" _color :!class /Script/Engine.MaterialInstanceDynamic))))
    (:then_1
      (Transformation|SetWorldLocation (Variables|Default|GetPhantom) (+ (Math|Vector|RotateVector (Variables|Default|GetPhantomLocation) (Transformation|GetActorRotation)) (Transformation|GetActorLocation)) false false)
      (Utilities|FlowControl|Sequence
        (:then_0
          (Transformation|SetWorldRotation _arrow (Math|Rotator|FindLookatRotation _returnvalue_2 _returnvalue) false false))
        (:then_1
          (Transformation|SetRelativeScale3D _arrow (Math|Vector|MakeVector (/ (Math|Vector|VectorLength (- _returnvalue_2 _returnvalue)) 1e+02) 3.0 3.0)))))))