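; BP_Porte is a placeable door that teleports the player when its wide arch wall mesh registers a hit.
; The hit moves player character 0 to the location and rotation of Billboard's root, without checking what struck the mesh.
; It then zeroes the character's movement velocity and resets the controller's rotation to zero, so the view ignores the destination's facing.
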(event OnComponentHit(SM_Wall_High_Sec1_Arch1_Wide)
  (params (HitComponent :type Primitive%20Component%20Object%20Reference) (OtherActor :type Actor%20Object%20Reference) (OtherComp :type Primitive%20Component%20Object%20Reference) (NormalImpulse :type Vector :default "0, 0, 0") (Hit :type Hit%20Result%20Structure%20%28by%20ref%29))
  (bind _returnvalue (Game|GetPlayerCharacter 0))
  (bind _billboard (Variables|Default|GetBillboard))
  (bind _rootcomponent (Variables|/Script/Engine.Actor|GetRootComponent _billboard))
  (bind _returnvalue_2 (Transformation|GetWorldTransform _rootcomponent))
  (Utilities|FlowControl|Sequence
    (:then_0
      (Transformation|SetActorLocationAndRotation _returnvalue (.location _returnvalue_2) (.rotation _returnvalue_2))
      (Variables|/Script/Engine.MovementComponent|SetVelocity (Variables|/Script/Engine.Character|GetCharacterMovement _returnvalue) "0, 0, 0"))
    (:then_1
      (Pawn|SetControlRotation (Game|GetPlayerController 0) (Math|Rotator|MakeRotator 0.0 0.0 0.0)))))

(fn ConstructionScript)