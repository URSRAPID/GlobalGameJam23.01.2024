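; BP_Test is a test actor that climbs steadily along world Z while printing its height.
; The construction script caches the actor's starting location in VLocation.
; Each Tick calls AddOffset, which moves the actor one unit up from the cached location without sweep and updates the cache, then prints the current Z.
; Movement is per frame with no delta-time scaling, so its speed depends on frame rate.
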(event EventTick
  (params (DeltaSeconds :type Float%20%28single-precision%29))
  (Utilities|FlowControl|Sequence
    (:then_0
      ;[1 0.4174 0] Print String
      (|AddOffset))
    (:then_1
      (Development|PrintString (Utilities|String|ToString(Float) (.z (Transformation|GetActorLocation)))))))

(fn ConstructionScript
  (Variables|Default|SetV_Location (Transformation|GetActorLocation)))