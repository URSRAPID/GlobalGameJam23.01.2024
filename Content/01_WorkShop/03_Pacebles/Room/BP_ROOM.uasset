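; BP_ROOM is a room actor whose cube kills the player character on contact.
; On BeginPlay it caches the player C_Perso and the HUD_WorkShop.
; A hit on SM_Cube by a living C_Perso sets IsDead, then turns on the cached player's physics mesh, passing this room's Billboard, and activates the HUD continue screen.
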(event OnComponentHit(SM_Cube)
  (params (HitComponent :type Primitive%20Component%20Object%20Reference) (OtherActor :type Actor%20Object%20Reference) (OtherComp :type Primitive%20Component%20Object%20Reference) (NormalImpulse :type Vector :default "0, 0, 0") (Hit :type Hit%20Result%20Structure%20%28by%20ref%29))
  (bind _asc_perso (Utilities|Casting|CastToC_Perso OtherActor))
  (if (not (Variables|/Game/01_WorkShop/02_Core/C_Perso.C_Perso_C|GetIsDead _asc_perso))
    (Variables|/Game/01_WorkShop/02_Core/C_Perso.C_Perso_C|SetIsDead _asc_perso true)
    (Utilities|FlowControl|Sequence
      (:then_0
        (Default|ActivatePhysicMesh (Variables|Default|GetAs%20C%20Perso) true (Variables|Default|GetBillboard)))
      (:then_1
        (Default|ActivationContinueScreen (Variables|Default|GetAs%20HUD%20Wark%20Shop) true)))))

(event EventBeginPlay
  (Utilities|FlowControl|Sequence
    (:then_0
      (bind _asc_perso (Utilities|Casting|CastToC_Perso (Game|GetPlayerCharacter 0)))
      (Variables|Default|SetAs%20C%20Perso _asc_perso))
    (:then_1
      (bind _ashud_work_shop (Utilities|Casting|CastToHUD_WorkShop (HUD|GetHUD (Game|GetPlayerController 0))))
      (Variables|Default|SetAs%20HUD%20Wark%20Shop _ashud_work_shop))))

(fn ConstructionScript)