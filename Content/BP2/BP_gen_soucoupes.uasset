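; BP_gen_soucoupes is a generator actor that spawns a grid of BP_soucoupe saucers and relays their destruction events with a score.
; On BeginPlay, nested loops spawn a three-by-three grid in the X-Z plane, offset from the generator's location.
; It binds to each saucer's EDestruction dispatcher and rebroadcasts the score through its own EDestruction, so listeners need only the generator.
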(event Custom|CustomEvent_1
  (params (I_Score :type Integer))
  (Default|CallEDestruction I_Score))

(event EventBeginPlay
  (bind _returnvalue (Transformation|GetActorLocation))
  (for _index (range 0 2)
    (for _index_2 (range 0 2)
      (bind _returnvalue_2 (Game|SpawnActorfromClass "/Game/BP2/BP_soucoupe.BP_soucoupe_C" (Math|Transform|MakeTransform (Math|Vector|MakeVector (+ (.x _returnvalue) (+ (Math|Conversions|ToFloat(Integer) (* _index 200)) 1.0)) (.y _returnvalue) (+ (.z _returnvalue) (+ (Math|Conversions|ToFloat(Integer) (* _index_2 200)) 1.0))) "0, 0, 0" "1,1,1") "Undefined" 0 0))
      (EventDispatchers|BindEventtoEDestruction _returnvalue_2 (delegate Custom|CustomEvent_1)))))

(event Collision|EventActorBeginOverlap
  (params (OtherActor :type Actor%20Object%20Reference)))

(event EventTick
  (params (DeltaSeconds :type Float%20%28single-precision%29)))

(fn ConstructionScript)