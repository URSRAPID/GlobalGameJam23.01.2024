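; BP_POOL_3 is an actor Blueprint that animates the relative position of its SMFan01 component.
; On BeginPlay it plays a timeline whose TrackX and TrackY outputs set the component's X and Y location on each update, with Z held at zero and no sweep.
; Tick, overlap and construction script add no logic of their own.
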(event EventBeginPlay
  (|CallParentFunction)
  (bind (_direction _track_x _track_y) (Timeline|Timeline_0 Play)
    (:Update
      (Transformation|SetRelativeLocation (Variables|Default|GetSM_Fan_01) (Math|Vector|MakeVector _track_x _track_y 0.0) false false))))

(event Collision|EventActorBeginOverlap
  (params (OtherActor :type Actor%20Object%20Reference))
  (|CallParentFunction OtherActor) ; This node is disabled and will not be called.\nDrag off pins to build functionality.
)

(event EventTick
  (params (DeltaSeconds :type Float%20%28single-precision%29))
  (|CallParentFunction DeltaSeconds) ; This node is disabled and will not be called.\nDrag off pins to build functionality.
)

(fn ConstructionScript
  (|CallParentFunction))