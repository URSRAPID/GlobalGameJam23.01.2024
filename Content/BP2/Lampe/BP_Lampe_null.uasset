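; Lamp actor whose point light toggles on and off when its switch mesh is clicked.
; BeginPlay enables input and click events on the first player controller.
; Box overlap sets a collision flag that gates the click, shows the cursor and switches to game-and-UI input, and end overlap reverts all three without filtering the overlapping actor.
; FAllumer and FEteindre set the light's visibility and the on/off state.
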(event OnComponentBeginOverlap(Box)
  (params (OverlappedComponent :type Primitive%20Component%20Object%20Reference) (OtherActor :type Actor%20Object%20Reference) (OtherComp :type Primitive%20Component%20Object%20Reference) (OtherBodyIndex :type Integer) (bFromSweep :type Boolean) (SweepResult :type Hit%20Result%20Structure%20%28by%20ref%29))
  (bind _returnvalue (Game|GetPlayerController 0))
  (Variables|Default|Setb_est_collision true)
  (Variables|/Script/Engine.PlayerController|SetbShowMouseCursor _returnvalue true)
  (Input|SetInputModeGameandUI _returnvalue 0 "DoNotLock" true))

(event OnComponentEndOverlap(Box)
  (params (OverlappedComponent :type Primitive%20Component%20Object%20Reference) (OtherActor :type Actor%20Object%20Reference) (OtherComp :type Primitive%20Component%20Object%20Reference) (OtherBodyIndex :type Integer))
  (bind _returnvalue (Game|GetPlayerController 0))
  (Variables|Default|Setb_est_collision false)
  (Variables|/Script/Engine.PlayerController|SetbShowMouseCursor _returnvalue false)
  (Input|SetInputModeGameOnly _returnvalue))

(event OnClicked(SM_intrerupteur)
  (params (TouchedComponent :type Primitive%20Component%20Object%20Reference) (ButtonPressed :type Key%20Structure))
  (if (Variables|Default|Getb_est_collision)
    (if (Variables|Default|Getb_est_allumer)
      (CallFunction|FEteindre)
      (else
        (CallFunction|FAllumer)))))

(event EventBeginPlay
  (bind _returnvalue (Game|GetPlayerController 0))
  (Input|EnableInput _returnvalue)
  (Variables|/Script/Engine.PlayerController|SetbEnableClickEvents _returnvalue true))

(event Collision|EventActorBeginOverlap
  (params (OtherActor :type Actor%20Object%20Reference)))

(event EventTick
  (params (DeltaSeconds :type Float%20%28single-precision%29)))

(fn ConstructionScript)

(fn FAllumer
  (Rendering|SetVisibility (Variables|Default|GetPointLight) true false)
  (Variables|Default|Setb_est_allumer true))

(fn FEteindre
  (Rendering|SetVisibility (Variables|Default|GetPointLight) false false)
  (Variables|Default|Setb_est_allumer false))