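; BP_Balle is a ball or bullet actor that removes itself after a limited lifetime.
; Each Tick calls DestroyBalle, which decrements the ITimeBalle counter.
; Once the counter reaches zero, further decrements drive a Lerp that shrinks the actor uniformly to nothing before it is destroyed.
; Lifetime and shrink are counted in frames rather than seconds, so their duration depends on frame rate.
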(event EventTick
  (params (DeltaSeconds :type Float%20%28single-precision%29))
  (CallFunction|DestroyBalle))

(fn ConstructionScript)

(fn DestroyBalle
  (bind _i_time_balle (Variables|Default|GetI_Time_balle))
  (bind _returnvalue (Math|Conversions|ToFloat(Integer) _i_time_balle))
  (bind _returnvalue_2 (/ _returnvalue -5e+01))
  (bind _returnvalue_3 (Math|Float|Lerp 0.25 0.0 _returnvalue_2))
  (Math|Integer|DecrementInt _i_time_balle
    (:%20%20
      (if (<= _i_time_balle 0)
        (if (<= _i_time_balle -50)
          (Actor|DestroyActor)
          (else
            (Transformation|SetActorScale3D (Math|Vector|MakeVector _returnvalue_3 _returnvalue_3 _returnvalue_3))))))))