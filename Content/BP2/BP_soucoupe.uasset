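; Flying saucer target that spins its crown mesh each tick and can be shot down by BP_Balle hits.
; Each hit decrements INbPas, playing a small explosion, or a larger one at zero before broadcasting EDestruction with its score and destroying itself.
; Explosion sounds play at world origin, not the hit location.
; An up/down bobbing function exists but is never called here, and reuses INbPas as its step counter.
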(event EventBeginPlay)

(event Collision|EventActorBeginOverlap
  (params (OtherActor :type Actor%20Object%20Reference)))

(event EventTick
  (params (DeltaSeconds :type Float%20%28single-precision%29))
  (CallFunction|FRotation))

(event Collision|EventHit
  (params (MyComp :type Primitive%20Component%20Object%20Reference) (Other :type Actor%20Object%20Reference) (OtherComp :type Primitive%20Component%20Object%20Reference) (bSelfMoved :type Boolean) (HitLocation :type Vector :default "0, 0, 0") (HitNormal :type Vector :default "0, 0, 0") (NormalImpulse :type Vector :default "0, 0, 0") (Hit :type Hit%20Result%20Structure%20%28by%20ref%29))
  (bind _i_nb_pas (Variables|Default|GetI_nb_pas))
  (Utilities|Casting|CastToBP_Balle Other)
  (Math|Integer|DecrementInt _i_nb_pas
    (:%20%20
      (if (<= _i_nb_pas 0)
        (Effects|SpawnEmitteratLocation "/Game/StarterContent/Particles/P_Explosion.P_Explosion" HitLocation)
        (Audio|PlaySoundatLocation "/Game/StarterContent/Audio/Explosion_Cue.Explosion_Cue" "0, 0, 0" "0, 0, 0" 1.0 1.0 0.0 0 0 0)
        (Default|CallEDestruction (Variables|Default|GetI_nb_Score))
        (Actor|DestroyActor)
        (else
          (Effects|SpawnEmitteratLocation "/Game/StarterContent/Particles/P_Explosion_2.P_Explosion_2" HitLocation)
          (Audio|PlaySoundatLocation "/Game/StarterContent/Audio/Explosion_Cue_curte.Explosion_Cue_curte" "0, 0, 0" "0, 0, 0" 1.0 1.0 0.0 0 0 0))))))

(fn ConstructionScript)

(fn FMonterDescende
  (bind _i_nb_pas (Variables|Default|GetI_nb_pas))
  (if (Variables|Default|GetIsGoingUp)
    (Math|Integer|IncrementInt _i_nb_pas
      (:%20%20
        (Transformation|AddRelativeLocation (Variables|Default|GetDefaultSceneRoot) "0,0.000000,5.000000" false false)
        (if (>= _i_nb_pas 50)
          (Variables|Default|SetIsGoingUp false))))
    (else
      (Math|Integer|DecrementInt _i_nb_pas
        (:%20%20
          (Transformation|AddRelativeLocation (Variables|Default|GetDefaultSceneRoot) "0, 0,-5.000000" false false)
          (if (<= _i_nb_pas -50)
            (Variables|Default|SetIsGoingUp true)))))))

(fn FRotation
  (Transformation|AddLocalRotation (Variables|Default|GetMesh_couronne) "0,10.000000, 0" false false))