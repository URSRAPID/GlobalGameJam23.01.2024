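; BP_Porte is a clickable door that swings open or shut while something overlaps the actor.
; Overlap shows the mouse cursor and enables Game and UI input; leaving restores game-only input and closes the door if open.
; FGestionPorte checks the overlap and open flags, then snaps the mesh 90 degrees via relative rotation.
; Helper names are inverted: FOvrirPorte clears the open flag, FFermerPorte sets it.
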(event EventBeginPlay
  (bind _returnvalue (Game|GetPlayerController 0))
  (Input|EnableInput _returnvalue)
  (Variables|/Script/Engine.PlayerController|SetbEnableClickEvents _returnvalue true))

(event Collision|EventActorBeginOverlap
  (params (OtherActor :type Actor%20Object%20Reference))
  (bind _returnvalue (Game|GetPlayerController 0))
  (Variables|Default|Setb_porte_collision true)
  (Variables|/Script/Engine.PlayerController|SetbShowMouseCursor _returnvalue true)
  (Input|SetInputModeGameandUI _returnvalue 0 "DoNotLock" true))

(event EventTick
  (params (DeltaSeconds :type Float%20%28single-precision%29)))

(event MouseInput|EventActorOnClicked
  (params (ButtonPressed :type Key%20Structure))
  (CallFunction|FGestionPorte))

(event Collision|EventActorEndOverlap
  (params (OtherActor :type Actor%20Object%20Reference))
  (bind _returnvalue (Game|GetPlayerController 0))
  (Variables|Default|Setb_porte_collision false)
  (Variables|/Script/Engine.PlayerController|SetbShowMouseCursor _returnvalue false)
  (Input|SetInputModeGameOnly _returnvalue)
  (CallFunction|FGestionPorte))

(event Input|ActionEvents|InputActionOvirirPorte
  (params (Key :type Key%20Structure))
  ;[1 1 1] Ovrir poirte
)

(fn ConstructionScript)

(fn FGestionPorte
  (if (Variables|Default|Getb_porte_collision)
    (if (Variables|Default|Getb_porte_ouverte)
      (CallFunction|FOvrirPorte :!label _label)
      (else
        (CallFunction|FFermerPorte)))
    (elif (Variables|Default|Getb_porte_ouverte)
      (goto _label))))

(fn FOvrirPorte
  (Transformation|AddRelativeRotation (Variables|Default|GetSM_porte) "0,-90.000000, 0" false false)
  (Variables|Default|Setb_porte_ouverte false))

(fn FFermerPorte
  (Transformation|AddRelativeRotation (Variables|Default|GetSM_porte) "0,90.000000, 0" false false)
  (Variables|Default|Setb_porte_ouverte true))