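; BP_Object is a scoring object that awards points when its static mesh is displaced from its starting position.
; BeginPlay records the mesh's world location and caches the player's HUD_test HUD.
; While active, Tick checks the distance from that origin; once it passes a small threshold, the object deactivates and adds its Value to the HUD score, so it scores only once.
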(event EventBeginPlay
  (Variables|Default|SetOriginLocation (Transformation|GetWorldLocation (Variables|Default|GetStaticMesh)))
  (bind _ashud_test (Utilities|Casting|CastToHUD_test (HUD|GetHUD (Game|GetPlayerController 0))))
  (Variables|Default|SetHUD%20Test _ashud_test))

(event EventTick
  (params (DeltaSeconds :type Float%20%28single-precision%29))
  (bind _hud_test (Variables|Default|GetHUD%20Test))
  (if (Variables|Default|GetbIsActive)
    (if (> (Math|Vector|Distance(Vector) (Variables|Default|GetOriginLocation) (Transformation|GetWorldLocation (Variables|Default|GetStaticMesh))) 1e+01)
      (Variables|Default|SetbIsActive false)
      (Utilities|IsValid _hud_test
        (:Is%20Valid
          (Default|AddScore _hud_test (Variables|Default|GetValue)))))))

(fn ConstructionScript)